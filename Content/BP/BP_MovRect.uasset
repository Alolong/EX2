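; BP_MovRect is an actor whose Cube component travels around a square path in its local X-Z plane while Isplay is true.
; Tick switches on the ENMove enum (Right, Up, Left, Down), stepping position a fixed amount per frame, independent of delta time, and changing direction past each bound.
; EventOverlap sets Isplay and returns false.
; Distance and Movereset maintain a Movedistance counter that the movement logic does not use.
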(event `self.ReceiveTick`
  (params (DeltaSeconds :type "Float (single-precision)"))
  (if (`self.isplay`)
    (switch `/Game/BP/EN_Move` (`self.EN_Move`)
      (:`NewEnumerator0`
        ; 오른쪽 이동
        (bind _output_get (set `self.X-move` (+ (`self.X-move`) 10.0)))
        (`SceneComponent.K2_SetRelativeLocation` (`self.Cube`) (`KismetMathLibrary.MakeVector` _output_get 0.0 (`self.z-move`)) false false)
        (if (> (`self.x-move`) 500.0)
          (set `self.EN_Move` "NewEnumerator1")))
      (:`NewEnumerator1`
        ; 위쪽
        (bind _output_get_2 (set `self.z-move` (+ (`self.z-move`) 10.0)))
        (`SceneComponent.K2_SetRelativeLocation` (`self.Cube`) (`KismetMathLibrary.MakeVector` (`self.x-move`) 0.0 _output_get_2) false false)
        (if (> (`self.z-move`) 500.0)
          (set `self.EN_Move` "NewEnumerator2")))
      (:`NewEnumerator2`
        ; 왼쪽이동
        (bind _output_get_3 (set `self.X-move` (+ (`self.X-move`) -10.0)))
        (`SceneComponent.K2_SetRelativeLocation` (`self.Cube`) (`KismetMathLibrary.MakeVector` _output_get_3 0.0 (`self.z-move`)) false false)
        (if (< (`self.x-move`) 0.0)
          (set `self.EN_Move` "NewEnumerator3")))
      (:`NewEnumerator3`
        ; 아래쪽
        (bind _output_get_4 (set `self.z-move` (+ (`self.z-move`) -10.0)))
        (`SceneComponent.K2_SetRelativeLocation` (`self.Cube`) (`KismetMathLibrary.MakeVector` (`self.x-move`) 0.0 _output_get_4) false false)
        (if (< (`self.z-move`) 0.0)
          (set `self.EN_Move` "NewEnumerator0"))))))

(fn `distance`
  (set `self.Movedistance` (+ (`self.Movedistance`) 10.0)))

(fn `EventOverlap`
  (params (isplay :type Boolean))
  (returns (return :type Boolean))
  (set `self.isplay` isplay)
  (return false))

(fn `Movereset`
  (if (>= (`self.Movedistance`) 500.0)
    (set `self.Movedistance` 0.0)))

(fn `UserConstructionScript`)
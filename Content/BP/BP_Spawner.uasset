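; BP_Spawner is an actor that scatters a batch of spawned actors, apparently coins, inside a box volume.
; EventOverlap calls DoSpawn when passed a true Isplay flag and returns false.
; DoSpawn loops up to Coinnumber, spawning the Spawn class at random points within the Box, multiplying its already scaled extent by actor scale.
; A disconnected branch that would pass Coinget to BP_Coin's Beginget never runs.
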(event `DoSpawn`
  (bind _box (`self.Box`))
  (for _ (range (+ (`self.Coinnumber`) 1))
    (`|SpawnActorFromClass` (`self.spawn`) (`KismetMathLibrary.MakeTransform` (`KismetMathLibrary.RandomPointInBoundingBox` (`SceneComponent.K2_GetComponentLocation` _box) (* (`BoxComponent.GetScaledBoxExtent` _box) (`self.GetActorScale3D`)))) "Undefined" "MultiplyWithRoot" null null)))

(fn `EventOverlap`
  (params (isplay :type Boolean))
  (returns (return :type Boolean))
  (if isplay
    (`self.DoSpawn`)
    (return false)))

(fn `UserConstructionScript`)
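; BP_timer is a stopwatch actor that shows elapsed play time on the HUD.
; While its running flag is set, Tick adds delta seconds to a counter and sends a zero-padded minutes:seconds string to BP_Hud's UpdateTime.
; EventOverlap sets the running flag from its input, starting or pausing the count without resetting it.
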(event `self.ReceiveTick`
  (params (DeltaSeconds :type "Float (single-precision)"))
  (if (`self.isruning`)
    ; 증가식
    (bind _output_get (set `self.countsecond` (+ DeltaSeconds (`self.countsecond`))))
    ; 캐스트
    (bind _asbp_hud (cast `/Game/BP/BP_Hud` (`PlayerController.GetHUD` (`GameplayStatics.GetPlayerController` 0))))
    (`/Game/BP/BP_Hud.UpdateTime` _asbp_hud (`KismetStringLibrary.Concat_StrStr` (`self.floortime` (/ _output_get 60.0)) ":" (`self.floortime` (mod _output_get 60.0))))))

(fn `EventOverlap`
  (params (isplay :type Boolean))
  (returns (return :type Boolean))
  (set `self.isruning` isplay)
  (return false))

(fn `floortime`
  (params (A :type "Float (double-precision)"))
  (returns (NewParam :type String))
  (bind _returnvalue (`KismetStringLibrary.Conv_IntToString` (`KismetMathLibrary.FFloor` A)))
  (if (< A 10.0)
    (return (`KismetStringLibrary.Concat_StrStr` "0" _returnvalue))
    (else
      (return _returnvalue))))

(fn `UserConstructionScript`)
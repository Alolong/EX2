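; BP_SplineMove is an actor that moves a cube along its spline continuously, starting at BeginPlay.
; A timeline value, scaled by spline length, samples the world transform at that distance and sets the cube's location and rotation each update, restarting from the start when finished.
; An unconnected back-and-forth variant, toggling an Isright flag to play or reverse a second timeline, remains in the graph but never runs.
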(event `self.ReceiveBeginPlay`
  (bind _spline (`self.Spline`))
  ; 반복
  (bind (_direction _value) (`Timeline|Timeline_0` :!label _label)
    (:`Update`
      (bind (_returnvalue_location _returnvalue_rotation) (`KismetMathLibrary.BreakTransform` (`SplineComponent.GetTransformAtDistanceAlongSpline` _spline (* _value (`SplineComponent.GetSplineLength` _spline)) "World" false)))
      (`SceneComponent.K2_SetWorldLocationAndRotation` (`self.Cube`) _returnvalue_location _returnvalue_rotation false false))
    (:`Finished`
      (goto _label :!via `PlayFromStart`))))

(fn `UserConstructionScript`)
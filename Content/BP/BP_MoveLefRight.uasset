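; BP_MoveLefRight is a Blueprint that slides its Cube component back and forth along the relative X axis while Isplay is true.
; Tick moves it by a fixed step per frame, so speed depends on frame rate, and flips the End direction flag whenever Movedistance reaches its limit.
; The EventOverlap function sets Isplay from its input to start or pause the motion, and always returns false.
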(event `self.ReceiveTick`
  (params (DeltaSeconds :type "Float (single-precision)"))
  (if (`self.isplay`)
    (set `self.Movedistance` (+ (`self.Movedistance`) 10.0))
    (if (`self.end`)
      (bind _output_get (set `self.X-move` (+ (`self.X-move`) 10.0)))
      (`SceneComponent.K2_SetRelativeLocation` (`self.Cube`) (`KismetMathLibrary.MakeVector` _output_get) false false)
      (if (>= (`self.Movedistance`) 500.0)
        (set `self.Movedistance` 0.0)
        (set `self.end` false))
      (else
        (bind _output_get_2 (set `self.X-move` (- (`self.X-move`) 10.0)))
        (`SceneComponent.K2_SetRelativeLocation` (`self.Cube`) (`KismetMathLibrary.MakeVector` _output_get_2) false false)
        (if (>= (`self.Movedistance`) 500.0)
          (set `self.Movedistance` 0.0)
          (set `self.end` true))))))

(fn `EventOverlap`
  (params (isplay :type Boolean))
  (returns (return :type Boolean))
  (set `self.isplay` isplay)
  (return false))

(fn `UserConstructionScript`)